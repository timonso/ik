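; BP_targetPath is a path actor that moves a referenced TargetObject along its spline, starting at BeginPlay.
; A Timeline, with play rate set from Duration, maps its track to distance along the spline and updates the target's location and tangent-aligned rotation.
; When the timeline finishes, it reverses to send the target back along the path.
; The construction script snaps the target to the first spline point.
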(event `startAnimation`
  (bind _spline (`self.Spline`))
  (bind (_direction _spline_track) (`Timeline|Timeline` :!via `PlayFromStart` :!label _label)
    (:`Update`
      (bind _returnvalue (`KismetMathLibrary.Lerp` 0.0 (`SplineComponent.GetDistanceAlongSplineAtSplinePoint` _spline (- (`SplineComponent.GetNumberOfSplinePoints` _spline) 1)) _spline_track))
      (`self.K2_SetActorLocationAndRotation` (`self.targetObject`) (`SplineComponent.GetLocationAtDistanceAlongSpline` _spline _returnvalue "World") (`KismetMathLibrary.Conv_VectorToRotator` (`SplineComponent.GetTangentAtDistanceAlongSpline` _spline _returnvalue "World")) false false))
    (:`Finished`
      (`self.reverseAnimation`))))

(event `self.ReceiveBeginPlay`
  (`TimelineComponent.SetPlayRate` (`self.Timeline`) (/ 1.0 (`self.duration`)))
  (`self.startAnimation`))

(event `reverseAnimation`
  (goto _label :!via `Reverse`))

(fn `UserConstructionScript`
  (`self.K2_SetActorLocation` (`self.targetObject`) (`SplineComponent.GetLocationAtSplinePoint` (`self.Spline`) 0 "World") false false))